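; BP_TestCount is a test actor that runs a CPU-heavy workload every frame, apparently for profiling Blueprint cost.
; Tick calls FunctionInsights, which runs two nested loops that both use NumLoop as their upper bound.
; Each inner iteration divides two random floats and passes the result to Print String with screen output disabled, so the work grows with the square of NumLoop.
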(event `self.ReceiveTick`
  (params (DeltaSeconds :type "Float (single-precision)"))
  (`self.FunctionInsights`))

(fn `FunctionInsights`
  (bind _returnvalue (`KismetMathLibrary.RandomFloatInRange` 1.0 100.0))
  (for _ (range (+ (`self.NumLoop`) 1))
    (for _ (range (+ (`self.NumLoop`) 1))
      (set `self.NumA` _returnvalue)
      (set `self.NumB` _returnvalue)
      (set `self.Result` (/ (`self.NumA`) (`self.NumB`)))
      (`KismetSystemLibrary.PrintString` (`KismetStringLibrary.Conv_DoubleToString` (`self.Result`)) false))))

(fn `UserConstructionScript`)